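; BP_Tile is one segment of an infinite terrain, with a barrier that gates the player and scattered props.
; On BeginPlay it locks the barrier and calls PlaceActors for containers, sandbags, boxes, canisters and rocks.
; The player overlapping LockingVolume opens the barrier and turns it green; leaving restores collision and red.
; Reaching GarbageDestroyVolume asks InfiniteTerrainGameMode to spawn another tile, then destroys this one; GetAttachLocation exposes the AttachPoint transform.
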(event OnComponentBeginOverlap(LockingVolume)
  (params (OverlappedComponent :type Primitive%20Component%20Object%20Reference) (OtherActor :type Actor%20Object%20Reference) (OtherComp :type Primitive%20Component%20Object%20Reference) (OtherBodyIndex :type Integer) (bFromSweep :type Boolean) (SweepResult :type Hit%20Result%20Structure%20%28by%20ref%29))
  (Utilities|IsPlayerActor OtherActor)
  (CallFunction|Unlock))

(event OnComponentEndOverlap(LockingVolume)
  (params (OverlappedComponent :type Primitive%20Component%20Object%20Reference) (OtherActor :type Actor%20Object%20Reference) (OtherComp :type Primitive%20Component%20Object%20Reference) (OtherBodyIndex :type Integer))
  (Utilities|IsPlayerActor OtherActor)
  (CallFunction|Lock))

(event OnComponentBeginOverlap(GarbageDestroyVolume)
  (params (OverlappedComponent :type Primitive%20Component%20Object%20Reference) (OtherActor :type Actor%20Object%20Reference) (OtherComp :type Primitive%20Component%20Object%20Reference) (OtherBodyIndex :type Integer) (bFromSweep :type Boolean) (SweepResult :type Hit%20Result%20Structure%20%28by%20ref%29))
  (Utilities|IsPlayerActor OtherActor)
  (bind _asinfinite_terrain_game_mode (Utilities|Casting|CastToInfiniteTerrainGameMode (Game|GetGameMode)))
  (Default|SpawnTile _asinfinite_terrain_game_mode)
  (Actor|DestroyActor))

(event EventBeginPlay
  (CallFunction|Lock)
  (Class|Tile|PlaceActors "/Game/Dynamic/Terrain/Props/BP_Container.BP_Container_C" (Variables|Default|GetContainerSpawnInfo))
  (Class|Tile|PlaceActors "/Game/Dynamic/Terrain/Props/BP_Sandbags.BP_Sandbags_C" (Variables|Default|GetSandbagsSpawnInfo))
  (Class|Tile|PlaceActors "/Game/Dynamic/Terrain/Props/BP_Box.BP_Box_C" (Variables|Default|GetBoxSpawnInfo))
  (Class|Tile|PlaceActors "/Game/Dynamic/Terrain/Props/BP_Canister.BP_Canister_C" (Variables|Default|GetCanisterSpawnInfo))
  (Class|Tile|PlaceActors "/Game/Dynamic/Terrain/Props/BP_Rock1.BP_Rock1_C" (Variables|Default|GetRock1SpawnInfo))
  (Class|Tile|PlaceActors "/Game/Dynamic/Terrain/Props/BP_Rock2.BP_Rock2_C" (Variables|Default|GetRock2SpawnInfo))
  (Class|Tile|PlaceActors "/Game/Dynamic/Terrain/Props/BP_Rock3.BP_Rock3_C" (Variables|Default|GetRock3SpawnInfo)))

(event Collision|EventActorBeginOverlap
  (params (OtherActor :type Actor%20Object%20Reference)))

(event EventTick
  (params (DeltaSeconds :type Float%20%28single-precision%29)))

(fn ConstructionScript)

(fn GetAttachLocation
  (return (Transformation|GetWorldTransform (Variables|Default|GetAttachPoint))))

(fn Unlock
  (bind _barrier (Variables|Default|GetBarrier))
  (Collision|SetCollisionEnabled _barrier "NoCollision")
  (Rendering|Material|SetMaterial _barrier 0 "/Game/Dynamic/Terrain/MI_Barrier_Green.MI_Barrier_Green"))

(fn Lock
  (bind _barrier (Variables|Default|GetBarrier))
  (Collision|SetCollisionEnabled _barrier "QueryAndPhysics")
  (Rendering|Material|SetMaterial _barrier 0 "/Game/Dynamic/Terrain/MI_Barrier_Red.MI_Barrier_Red"))