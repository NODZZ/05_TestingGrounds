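; AI controller for guard NPCs that runs the GuardBehaviour behavior tree on the PatrolData blackboard.
; Perception updates set EnemyKey to any sensed actor not tagged "Enemy" and clear it when such an actor's stimulus is lost.
; Every tick, the pawn's Aiming and Shooting flags follow whether the controller has a valid focus actor, which this Blueprint never sets itself.
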(event OnTargetPerceptionUpdated(AIPerception)
  (params (Actor :type Actor%20Object%20Reference) (Stimulus :type AI%20Stimulus%20Structure))
  (CallFunction|UpdateBlackboardEnemyKey Stimulus Actor Actor))

(event EventBeginPlay
  (bind _blackboardcomponent (Class|AIController|UseBlackboard "/Game/Dynamic/Character/AI/PatrolData.PatrolData"))
  (AI|RunBehaviorTree "/Game/Dynamic/Character/AI/GuardBehaviour.GuardBehaviour")
  (Variables|Default|SetBlackboardComp _blackboardcomponent))

(event EventTick
  (params (DeltaSeconds :type Float%20%28single-precision%29))
  (CallFunction|SetAimingShooting))

(fn ConstructionScript)

(fn SetAimingShooting
  (bind _returnvalue (Class|AIController|GetFocusActor))
  (bind _returnvalue_2 (Utilities|IsValid _returnvalue))
  (bind _ascharacter (Utilities|Casting|CastToCharacter (Pawn|GetControlledPawn)))
  (Variables|/Game/Dynamic/Character/Behaviour/Character.Character_C|SetAiming _ascharacter _returnvalue_2)
  (Variables|/Game/Dynamic/Character/Behaviour/Character.Character_C|SetShooting _ascharacter _returnvalue_2))

(fn SetorClearEnemyKey
  (params (ObjectValue :type Object%20Object%20Reference) (Condition :type Boolean))
  (bind _enemykey (Variables|Default|GetEnemyKey))
  (bind _blackboardcomp (Variables|Default|GetBlackboardComp))
  (if Condition
    (AI|Components|Blackboard|SetValueasObject _blackboardcomp _enemykey ObjectValue)
    (else
      (AI|Components|Blackboard|ClearValue _blackboardcomp _enemykey))))

(fn UpdateBlackboardEnemyKey
  (params (AIStimulus :type AI%20Stimulus%20Structure%20%28by%20ref%29) (self2 :type Actor%20Object%20Reference) (ObjectValue :type Object%20Object%20Reference))
  (if (not (Actor|ActorHasTag self2 "Enemy"))
    (CallFunction|SetorClearEnemyKey ObjectValue (.bSuccessfullySensed (Utilities|Struct|BreakAIStimulus AIStimulus)))))